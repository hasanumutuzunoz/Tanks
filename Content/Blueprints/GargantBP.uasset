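; Gargant zombie enemy that supplies Paper2D flipbook visuals for the walk, attack and death events.
; Walk playback rate scales with movement speed between walk and run speeds, while attack restarts its own flipbook.
; Death plays a sound, disables collision, lowers the actor and drives a blue-boosted sprite alpha by timeline before destroying it.
; Crushed deaths also animate the flipbook's scale through a second timeline.
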(event EventBeginPlay)

(event Collision|EventActorBeginOverlap
  (params (OtherActor :type Actor%20Object%20Reference)))

(event EventTick
  (params (DeltaSeconds :type Float%20%28single-precision%29)))

(event EventZombieWalk
  (params (DeltaSeconds :type Float%20%28single-precision%29) (DistanceWalkedThisFrame :type Vector :default "0, 0, 0"))
  (Class|TankStatics|PlayFlipbook (Variables|Default|GetPaperFlipbook) "/Game/paperFlipbooks/gargant-move_gargant_move.gargant-move_gargant_move" true (Math|Float|MapRangeClamped (/ (Math|Vector|VectorLength DistanceWalkedThisFrame) DeltaSeconds) (Variables|Default|GetWalkSpeed) (Variables|Default|GetRunSpeed) 1.0 2.0) false))

(event EventZombieAttack
  (params (DeltaSeconds :type Float%20%28single-precision%29))
  (Class|TankStatics|PlayFlipbook (Variables|Default|GetPaperFlipbook) "/Game/paperFlipbooks/gargant-attack_Gargant_Attack.gargant-attack_Gargant_Attack" false 1.0 true))

(event EventZombieDie
  (params (DamageType :type EDamageType%20Enum :default "Unknown"))
  (bind _self self)
  (bind _paperflipbook (Variables|Default|GetPaperFlipbook))
  (Audio|PlaySound2D "/Game/Sounds/gargant_die.gargant_die" 1.0 1.0 0.0 0 0)
  (Collision|SetActorEnableCollision _self false)
  (Transformation|SetActorLocation (+ (Transformation|GetActorLocation) (Math|Vector|MakeVector 0.0 0.0 -1e+01)) false false)
  (Class|TankStatics|PlayFlipbook (Variables|Default|GetPaperFlipbook) "/Game/paperFlipbooks/Dead_gargant_Dead_Gargant.Dead_gargant_Dead_Gargant" false 1.0 true)
  (Utilities|FlowControl|Sequence
    (:then_0
      (bind _newtrack_0 (Timeline|Timeline_0 PlayFromStart)
        (:Update
          (Sprite|SetSpriteColor _paperflipbook (Utilities|Struct|MakeLinearColor 1.0 1.0 1e+02 _newtrack_0)))
        (:Finished
          (Actor|DestroyActor _self))))
    (:then_1
      (switch Utilities|FlowControl|Switch|SwitchonEDamageType DamageType
        (:Crushed
          (bind _newtrack_0_2 (Timeline|Timeline_1 Play)
            (:Update
              (Transformation|SetWorldScale3D _paperflipbook (Math|Conversions|ToVector(Float) _newtrack_0_2)))))))))

(fn ConstructionScript)