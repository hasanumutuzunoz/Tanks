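; RegularMissileBP is a missile Blueprint that handles how a regular missile explodes.
; On explode it plays a bang sound, starts a one-shot explosion flipbook, clears the missile sprite and sets its speed to zero.
; It defers the parent class's explode logic until the flipbook finishes playing, using a bound finished-playing event.
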(event Custom|FinishExploding
  (|CallParentFunction))

(event EventBeginPlay)

(event Collision|EventActorBeginOverlap
  (params (OtherActor :type Actor%20Object%20Reference)))

(event EventTick
  (params (DeltaSeconds :type Float%20%28single-precision%29)))

(event EventOnExplode
  (bind _paperflipbook (Variables|Default|GetPaperFlipbook))
  (Audio|PlaySound2D "/Game/Sounds/qubodup-BangMid.qubodup-BangMid" 0.4 1.0 0.0 0 0)
  (Sprite|SetFlipbook _paperflipbook "/Game/paperFlipbooks/explosion.explosion")
  (Audio|Components|Audio|Play _paperflipbook)
  (Components|Timeline|SetLooping _paperflipbook false)
  (EventDispatchers|BindEventtoOnFinishedPlaying _paperflipbook (delegate Custom|FinishExploding))
  (Rendering|Components|Sprite|SetSprite (Variables|Default|GetPaperSprite) 0)
  (Variables|Default|SetSpeed 0.0))

(fn ConstructionScript)